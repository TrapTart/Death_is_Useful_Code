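; BP_Pit is a death pit that also handles spawning the player in a side-scroller level.
; On BeginPlay it finds the BP_LevelCamera, spawns a SideScrollerCharacter at its Sphere's location, then looks up the "Player"-tagged character and hands it to the camera.
; When that character overlaps the Death component, the pit destroys it, spawns a replacement the same way and sets the camera's CanJump to true.
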(event `self.ReceiveBeginPlay`
  (bind _outactors (`GameplayStatics.GetAllActorsOfClass` "/Game/Blueprints/BP_LevelCamera.BP_LevelCamera_C"))
  (set `self.PCamera` (`|GetArrayItem` _outactors))
  (`self.SetPlayer`))

(event `self.Death.OnComponentBeginOverlap`
  (params (OverlappedComponent :type "PrimitiveComponent Object Reference") (OtherActor :type "Actor Object Reference") (OtherComp :type "PrimitiveComponent Object Reference") (OtherBodyIndex :type Integer) (bFromSweep :type Boolean) (SweepResult :type "HitResult Structure (by ref)"))
  (if (== OtherActor (`self.PCharacter`))
    (`self.K2_DestroyActor` (`self.PCharacter`))
    (`self.SetPlayer`)
    (set `/Game/Blueprints/BP_LevelCamera.canJump?` true (`self.PCamera`))))

(fn `SetPlayer`
  (`|SpawnActorFromClass` "/Game/Blueprints/SideScrollerCharacter.SideScrollerCharacter_C" (`KismetMathLibrary.MakeTransform` (`SceneComponent.K2_GetComponentLocation` (`self.Sphere`)) (struct :`Yaw` 90.0)) "AdjustIfPossibleButAlwaysSpawn" "OverrideRootScale" null null)
  (bind _outactors (`GameplayStatics.GetAllActorsOfClassWithTag` "/Game/Blueprints/SideScrollerCharacter.SideScrollerCharacter_C" "Player"))
  (bind _output_get (set `self.PCharacter` (`|GetArrayItem` _outactors)))
  (set `/Game/Blueprints/BP_LevelCamera.PCharacter` _output_get (`self.PCamera`)))

(fn `UserConstructionScript`)