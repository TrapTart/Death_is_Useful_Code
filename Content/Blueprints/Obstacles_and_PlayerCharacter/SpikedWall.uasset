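; Spiked wall obstacle that kills the side-scroller player on Box overlap, and also spawns the player at its Sphere on BeginPlay and after death.
; SetPlayer passes the tagged character to the level camera.
; While Numdied is below one (never incremented here), death plays a two-line typewriter speech with talking audio before respawning and enabling camera turning.
; When writing finishes, the audio stops and the HUD appears.
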(event `self.ReceiveBeginPlay`
  (bind _outactors (`GameplayStatics.GetAllActorsOfClass` "/Game/Blueprints/Obstacles_and_PlayerCharacter/BP_LevelCamera.BP_LevelCamera_C"))
  (set `self.PCamera` (`|GetArrayItem` _outactors))
  (`self.SetPlayer`))

(event `self.Box.OnComponentBeginOverlap`
  (params (OverlappedComponent :type "PrimitiveComponent Object Reference") (OtherActor :type "Actor Object Reference") (OtherComp :type "PrimitiveComponent Object Reference") (OtherBodyIndex :type Integer) (bFromSweep :type Boolean) (SweepResult :type "HitResult Structure (by ref)"))
  (bind _pcharacter (`self.PCharacter`))
  (if (== OtherActor _pcharacter)
    (`/Game/Blueprints/Obstacles_and_PlayerCharacter/SideScrollerCharacter.Death` _pcharacter false 0.0)
    (`KismetSystemLibrary.RetriggerableDelay` 2.0)
    (`self.K2_DestroyActor` (`self.PCharacter`))
    (if (not (>= (`self.numdied`) 1))
      (bind _returnvalue (`|CreateWidget` "/Game/Blueprints/UI/TypeWriterWidget.TypeWriterWidget_C" (`GameplayStatics.GetPlayerController` 0) "" 35.0))
      (`UserWidget.AddToViewport` _returnvalue 0)
      (bind _returnvalue_2 (`GameplayStatics.CreateSound2D` "/Game/Blueprints/Assets/Talking.Talking" 1.0 1.0 0.0 null))
      (`AudioComponent.Play` _returnvalue_2 0.0)
      (`/Game/Blueprints/UI/TypeWriterWidget.Write` _returnvalue (`|GetArrayItem` (`self.Speech`)))
      (`KismetSystemLibrary.Delay` 4.0)
      (`/Game/Blueprints/UI/TypeWriterWidget.Write` _returnvalue (`|GetArrayItem` (`self.Speech`) 1))
      (add `/Game/Blueprints/UI/TypeWriterWidget.FinshedWriting` _returnvalue (delegate `FinshedWriting_Event_0`))
      (`self.SetPlayer`)
      (set `/Game/Blueprints/Obstacles_and_PlayerCharacter/BP_LevelCamera.canTurn?` true (`self.PCamera`))
      (else
        (`self.SetPlayer`)))))

(event `FinshedWriting_Event_0`
  (`KismetSystemLibrary.Delay` 2.0)
  (`AudioComponent.Stop` (stale `self.Box.OnComponentBeginOverlap` _returnvalue_2))
  (`Widget.SetVisibility` (`/Game/Blueprints/UI/AblitiesWidget.CanvasPanel_0` (`/Game/Blueprints/Obstacles_and_PlayerCharacter/BP_LevelCamera.HUD` (`self.PCamera`))) "Visible")
  (`Widget.RemoveFromParent` (stale `self.Box.OnComponentBeginOverlap` _returnvalue)))

(fn `SetPlayer`
  (`|SpawnActorFromClass` "/Game/Blueprints/Obstacles_and_PlayerCharacter/SideScrollerCharacter.SideScrollerCharacter_C" (`KismetMathLibrary.MakeTransform` (`SceneComponent.K2_GetComponentLocation` (`self.Sphere`)) (struct :`Yaw` 90.0)) "AdjustIfPossibleButAlwaysSpawn" "OverrideRootScale" null null)
  (bind _outactors (`GameplayStatics.GetAllActorsOfClassWithTag` "/Game/Blueprints/Obstacles_and_PlayerCharacter/SideScrollerCharacter.SideScrollerCharacter_C" "Player"))
  (bind _output_get (set `self.PCharacter` (`|GetArrayItem` _outactors)))
  (set `/Game/Blueprints/Obstacles_and_PlayerCharacter/BP_LevelCamera.PCharacter` _output_get (`self.PCamera`)))

(fn `UserConstructionScript`)