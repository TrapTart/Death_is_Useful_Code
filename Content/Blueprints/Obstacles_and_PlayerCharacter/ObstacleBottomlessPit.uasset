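; Bottomless pit obstacle for the side-scroller that kills the player on overlap and spawns a replacement at its spawn point.
; When spawning is enabled, it also creates the player at BeginPlay and can set the jump at start, with the turn nested under that option.
; The box overlap calls Death with optional ragdoll, triggers text, respawns, sets jump and turn once only, then resets both UI counters.
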(event `self.ReceiveBeginPlay`
  (`parent.ReceiveBeginPlay`)
  (if (`self.isSpawning?`)
    (`self.SpawnNewPlayer` (`self.SpawnPoint`))
    (if (`self.JumpAtStart?`)
      (`self.Set the Jump`)
      (if (`self.TurnAtStart?`)
        (`self.Set the Turn`)))))

(event `self.Box.OnComponentBeginOverlap`
  (params (OverlappedComponent :type "PrimitiveComponent Object Reference") (OtherActor :type "Actor Object Reference") (OtherComp :type "PrimitiveComponent Object Reference") (OtherBodyIndex :type Integer) (bFromSweep :type Boolean) (SweepResult :type "HitResult Structure (by ref)"))
  (if (`self.ActorHasTag` OtherActor "Player")
    (`/Game/Blueprints/Obstacles_and_PlayerCharacter/SideScrollerCharacter.Death` (cast `/Game/Blueprints/Obstacles_and_PlayerCharacter/SideScrollerCharacter` OtherActor :!pure true) (`self.Is Ragdoll?`) 0.0)
    (`self.Text`)
    (`self.SpawnNewPlayer` (`self.SpawnPoint`))
    (`|ExecutionSequence`
      (:`then_0`
        (`/Engine/EditorBlueprintResources/StandardMacros.DoOnce` false
          (:`Completed`
            (`self.Set the Jump`)
            (`self.Set the Turn`))))
      (:`then_1`
        (`self.ResetJumps`)
        (`self.ResetTurns`)))))

(fn `UserConstructionScript`
  (`parent.UserConstructionScript`))