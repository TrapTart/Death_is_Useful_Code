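; Level camera Blueprint that handles player input and HUD for a side-scroller with limited jumps and turns, or shows the main menu when flagged.
; BeginPlay finds the tagged player character, stores its spawn point and fills the abilities HUD, zeroing displayed counts in tutorials.
; E starts movement, while Jump and Q spend charges to jump or flip direction.
; R clears dead characters, leaves the current one and spawns a replacement at the start.
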(event `self.ReceiveBeginPlay`
  (bind _returnvalue (`GameplayStatics.GetPlayerController` 0))
  (bind _hud (`self.HUD`))
  (bind _hud_2 (`self.HUD`))
  (if (`self.MainMenu?`)
    (bind _returnvalue_2 (`|CreateWidget` "/Game/Blueprints/UI/MainMenu.MainMenu_C"))
    (`UserWidget.AddToViewport` _returnvalue_2 0)
    (`WidgetBlueprintLibrary.SetInputMode_UIOnlyEx` _returnvalue null)
    (set `PlayerController.bShowMouseCursor` true _returnvalue)
    (else
      (bind _outactors (`GameplayStatics.GetAllActorsOfClassWithTag` "/Game/Blueprints/Obstacles_and_PlayerCharacter/SideScrollerCharacter.SideScrollerCharacter_C" "Player"))
      (bind _output (`|GetArrayItem` _outactors))
      (set `self.PCharacter` _output)
      (set `self.SpawnLocation` (`self.K2_GetActorLocation` _output))
      (bind _returnvalue_3 (`|CreateWidget` "/Game/Blueprints/UI/AblitiesWidget.AblitiesWidget_C"))
      (bind _output_get (set `self.HUD` _returnvalue_3))
      (`UserWidget.AddToViewport` _output_get 0)
      (`/Game/Blueprints/UI/AblitiesWidget.FadeIn` _output_get "Reverse" 2.0 "Visible")
      (bind _output_get_2 (set `self.Jumps` (`self.DefaultJumps`)))
      (bind _output_get_3 (set `self.Turns` (`self.DefaultTurns`)))
      (if (`self.isTutorialLevel?`)
        (`/Game/Blueprints/UI/AblitiesWidget.JumpsRemain` _hud 0)
        (`/Game/Blueprints/UI/AblitiesWidget.TurnsRemain` _hud 0)
        (else
          (`/Game/Blueprints/UI/AblitiesWidget.JumpsRemain` _hud_2 _output_get_2)
          (`/Game/Blueprints/UI/AblitiesWidget.TurnsRemain` _hud_2 _output_get_3))))))

(event `Key|E`
  (params (Key :type "Key Structure"))
  (:`Pressed`
    (`/Game/Blueprints/Obstacles_and_PlayerCharacter/SideScrollerCharacter.StartMovement` (`self.PCharacter`))))

(event `InputAction|Jump`
  (params (Key :type "Key Structure"))
  (bind _pcharacter (`self.PCharacter`))
  (:`Pressed`
    (if (> (`self.Jumps`) 0)
      (if (`self.canJump?`)
        (if (`Character.CanJump` (`self.PCharacter`))
          (`Character.Jump` _pcharacter)
          (bind _output_get (set `self.Jumps` (`KismetMathLibrary.Clamp` (- (`self.Jumps`) 1) 0 3)))
          (`/Game/Blueprints/UI/AblitiesWidget.JumpsRemain` (`self.HUD`) _output_get)))))
  (:`Released`
    (`Character.StopJumping` _pcharacter)))

(event `Key|Q`
  (params (Key :type "Key Structure"))
  (bind _hud (`self.HUD`))
  (bind _pcharacter (`self.PCharacter`))
  (bind _returnvalue (`KismetMathLibrary.Clamp` (- (`self.Turns`) 1) 0 6))
  (:`Pressed`
    (if (> (`self.Turns`) 0)
      (if (`self.canTurn?`)
        (`/Engine/EditorBlueprintResources/StandardMacros.FlipFlop`
          (:`A`
            (set `/Game/Blueprints/Obstacles_and_PlayerCharacter/SideScrollerCharacter.moveRight?` true _pcharacter)
            (bind _output_get (set `self.Turns` _returnvalue))
            (`/Game/Blueprints/UI/AblitiesWidget.TurnsRemain` _hud _output_get))
          (:`B`
            (set `/Game/Blueprints/Obstacles_and_PlayerCharacter/SideScrollerCharacter.moveRight?` false _pcharacter)
            (bind _output_get_2 (set `self.Turns` _returnvalue))
            (`/Game/Blueprints/UI/AblitiesWidget.TurnsRemain` _hud _output_get_2)))))))

(event `Key|R`
  (params (Key :type "Key Structure"))
  (:`Pressed`
    (bind _outactors (`GameplayStatics.GetAllActorsOfClassWithTag` "/Game/Blueprints/Obstacles_and_PlayerCharacter/SideScrollerCharacter.SideScrollerCharacter_C" "Dead"))
    (if (>= (`KismetArrayLibrary.Array_Length` _outactors) 1)
      (for _array_element _outactors
        (`self.K2_DestroyActor` _array_element)))
    (`/Game/Blueprints/Obstacles_and_PlayerCharacter/SideScrollerCharacter.LeaveCharacter` (`self.PCharacter`))
    (bind _returnvalue (`|SpawnActorFromClass` "/Game/Blueprints/Obstacles_and_PlayerCharacter/SideScrollerCharacter.SideScrollerCharacter_C" (`KismetMathLibrary.MakeTransform` (`self.SpawnLocation`) (struct :`Yaw` 90.0)) "AdjustIfPossibleButAlwaysSpawn" "OverrideRootScale" null null))
    (set `self.PCharacter` _returnvalue)))

(fn `UserConstructionScript`)