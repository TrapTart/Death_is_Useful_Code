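; Interactable is a trigger actor that moves a referenced object's static mesh along world X when the player overlaps its box.
; An overlap from a "Player"-tagged actor plays a timeline whose track drives a vector lerp toward a 250-unit X offset.
; Both lerp endpoints use the mesh's current location each update, so movement accumulates rather than stopping at 250 units.
; BeginPlay prints a warning if the Object reference is unset.
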(event `self.ReceiveBeginPlay`
  (`/Engine/EditorBlueprintResources/StandardMacros.IsValid` (`self.Object`)
    (:`Is Not Valid`
      (`KismetSystemLibrary.PrintString` "Set the Interactable Please"))))

(event `self.Box.OnComponentBeginOverlap`
  (params (OverlappedComponent :type "PrimitiveComponent Object Reference") (OtherActor :type "Actor Object Reference") (OtherComp :type "PrimitiveComponent Object Reference") (OtherBodyIndex :type Integer) (bFromSweep :type Boolean) (SweepResult :type "HitResult Structure (by ref)"))
  (bind _staticmesh (`/Game/Blueprints/Obstacles_and_PlayerCharacter/SpikedWall.StaticMesh` (`self.Object`)))
  (bind _returnvalue (`SceneComponent.K2_GetComponentLocation` _staticmesh))
  (if (`self.ActorHasTag` OtherActor "Player")
    (bind (_direction _newtrack_0) (`Timeline|Timelime`)
      (:`Update`
        (`SceneComponent.K2_SetWorldLocation` _staticmesh (`KismetMathLibrary.VLerp` _returnvalue (+ _returnvalue (250.0 0.0 0.0)) _newtrack_0) false false)))))

(fn `UserConstructionScript`)