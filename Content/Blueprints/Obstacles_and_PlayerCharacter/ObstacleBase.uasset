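; Base obstacle Blueprint with shared events for controlling the player's jump and turn abilities, respawning and dialogue.
; On BeginPlay it caches BP_LevelCamera and its starting Jumps and Turns, which reset events restore and push to the HUD.
; Other events copy CanJump and CanTurn to the camera or spawn a SideScrollerCharacter and assign it there.
; Text feeds Speech lines to a typewriter widget, removing it after a delay.
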(event `self.ReceiveBeginPlay`
  (bind _outactors (`GameplayStatics.GetAllActorsOfClass` "/Game/Blueprints/Obstacles_and_PlayerCharacter/BP_LevelCamera.BP_LevelCamera_C"))
  (bind _output_get (set `self.PCamera` (`|GetArrayItem` _outactors)))
  (set `self.DefaultJumps` (`/Game/Blueprints/Obstacles_and_PlayerCharacter/BP_LevelCamera.Jumps` _output_get))
  (set `self.DefaultTurns` (`/Game/Blueprints/Obstacles_and_PlayerCharacter/BP_LevelCamera.Turns` _output_get)))

(event `Set the Jump`
  (set `/Game/Blueprints/Obstacles_and_PlayerCharacter/BP_LevelCamera.canJump?` (`self.Can Jump?`) (`self.PCamera`)))

(event `SpawnNewPlayer`
  (params (SpawnLocation :type "SceneComponent Object Reference"))
  (`self.Spawn New Player` SpawnLocation))

(event `Text`
  (bind _returnvalue (`|CreateWidget` "/Game/Blueprints/UI/TypeWriterWidget.TypeWriterWidget_C" null "" 35.0))
  (for _array_element (`self.Speech`)
    (`UserWidget.AddToViewport` _returnvalue 0)
    (`/Game/Blueprints/UI/TypeWriterWidget.Write` _returnvalue _array_element)
    (`KismetSystemLibrary.RetriggerableDelay` 5.0))
  (`KismetSystemLibrary.Delay` 5.0)
  (`Widget.RemoveFromParent` _returnvalue))

(event `ResetJumps`
  (bind _pcamera (`self.PCamera`))
  (bind _output_get (set `/Game/Blueprints/Obstacles_and_PlayerCharacter/BP_LevelCamera.Jumps` (`self.DefaultJumps`) _pcamera))
  (`/Game/Blueprints/UI/AblitiesWidget.JumpsRemain` (`/Game/Blueprints/Obstacles_and_PlayerCharacter/BP_LevelCamera.HUD` _pcamera) _output_get))

(event `ResetTurns`
  (bind _pcamera (`self.PCamera`))
  (bind _output_get (set `/Game/Blueprints/Obstacles_and_PlayerCharacter/BP_LevelCamera.Turns` (`self.DefaultTurns`) _pcamera))
  (`/Game/Blueprints/UI/AblitiesWidget.TurnsRemain` (`/Game/Blueprints/Obstacles_and_PlayerCharacter/BP_LevelCamera.HUD` _pcamera) _output_get))

(event `Set the Turn`
  (set `/Game/Blueprints/Obstacles_and_PlayerCharacter/BP_LevelCamera.canTurn?` (`self.Can Turn?`) (`self.PCamera`)))

(fn `Spawn New Player`
  (params (SpawnLocation :type "SceneComponent Object Reference"))
  (bind _returnvalue (`|SpawnActorFromClass` "/Game/Blueprints/Obstacles_and_PlayerCharacter/SideScrollerCharacter.SideScrollerCharacter_C" (`KismetMathLibrary.MakeTransform` (`SceneComponent.K2_GetComponentLocation` SpawnLocation) (struct :`Yaw` 90.0)) "AdjustIfPossibleButAlwaysSpawn" "OverrideRootScale" null null))
  (set `/Game/Blueprints/Obstacles_and_PlayerCharacter/BP_LevelCamera.PCharacter` _returnvalue (`self.PCamera`)))

(fn `UserConstructionScript`)