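; Spike wall obstacle that kills the player on contact with its box and respawns them at a spawn point.
; Overlap with a Player-tagged actor calls Death on the SideScrollerCharacter with a ragdoll flag, then after a two-second delay calls Text, spawns a new player and resets jumps and turns.
; BeginPlay also spawns a player and initializes the jump and turn through SetTheJump and SetTheTurn.
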(event `self.ReceiveBeginPlay`
  (`parent.ReceiveBeginPlay`)
  (`self.SpawnNewPlayer` (`self.SpawnPoint`))
  (`self.Set the Jump`)
  (`self.Set the Turn`))

(event `self.Box.OnComponentBeginOverlap`
  (params (OverlappedComponent :type "PrimitiveComponent Object Reference") (OtherActor :type "Actor Object Reference") (OtherComp :type "PrimitiveComponent Object Reference") (OtherBodyIndex :type Integer) (bFromSweep :type Boolean) (SweepResult :type "HitResult Structure (by ref)"))
  (if (`self.ActorHasTag` OtherActor "Player")
    (`/Game/Blueprints/Obstacles_and_PlayerCharacter/SideScrollerCharacter.Death` (cast `/Game/Blueprints/Obstacles_and_PlayerCharacter/SideScrollerCharacter` OtherActor :!pure true) (`self.Is Ragdoll?`) 2.0)
    (`KismetSystemLibrary.Delay` 2.0)
    (`self.Text`)
    (`self.SpawnNewPlayer` (`self.SpawnPoint`))
    (`self.ResetJumps`)
    (`self.ResetTurns`)))

(fn `UserConstructionScript`
  (`parent.UserConstructionScript`))