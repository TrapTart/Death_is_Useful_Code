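; NextLevel is a level-transition trigger actor that opens the level given by LevelName when the player enters its Box.
; An overlap by an actor tagged "Player" plays the FadeOut level sequence, waits for its end time, then opens the level.
; Shortly after BeginPlay, SetPlayer caches the tagged SideScrollerCharacter in PCharacter, though the overlap logic does not use it.
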(event `self.ReceiveBeginPlay`
  (`KismetSystemLibrary.Delay` 0.5)
  (`self.SetPlayer`))

(event `self.Box.OnComponentBeginOverlap`
  (params (OverlappedComponent :type "PrimitiveComponent Object Reference") (OtherActor :type "Actor Object Reference") (OtherComp :type "PrimitiveComponent Object Reference") (OtherBodyIndex :type Integer) (bFromSweep :type Boolean) (SweepResult :type "HitResult Structure (by ref)"))
  (if (`self.ActorHasTag` OtherActor "Player")
    (bind _outactor (`LevelSequencePlayer.CreateLevelSequencePlayer` "/Game/Blueprints/FadeIn/FadeOut.FadeOut"))
    (bind _sequenceplayer (`LevelSequenceActor.SequencePlayer` _outactor))
    (`MovieSceneSequencePlayer.Play` _sequenceplayer)
    (`KismetSystemLibrary.Delay` (`TimeManagementBlueprintLibrary.Conv_QualifiedFrameTimeToSeconds` (`MovieSceneSequencePlayer.GetEndTime` _sequenceplayer)))
    (`GameplayStatics.OpenLevel` (`self.Level Name`))))

(fn `SetPlayer`
  (bind _outactors (`GameplayStatics.GetAllActorsOfClassWithTag` "/Game/Blueprints/Obstacles_and_PlayerCharacter/SideScrollerCharacter.SideScrollerCharacter_C" "Player"))
  (set `self.PCharacter` (`|GetArrayItem` _outactors)))

(fn `UserConstructionScript`)