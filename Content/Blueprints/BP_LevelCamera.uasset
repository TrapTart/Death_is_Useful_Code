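; BP_LevelCamera relays player input to the side-scroller character tagged "Player", which it finds and caches on BeginPlay.
; E starts the character's movement, and Q alternates its MoveRight flag through a FlipFlop when CanTurn is set.
; The Jump action starts a jump when CanJump is set and always stops it on release.
; Despite the name, the graphs contain no camera logic.
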(event `self.ReceiveBeginPlay`
  (bind _outactors (`GameplayStatics.GetAllActorsOfClassWithTag` "/Game/Blueprints/SideScrollerCharacter.SideScrollerCharacter_C" "Player"))
  (set `self.PCharacter` (`|GetArrayItem` _outactors)))

(event `Key|E`
  (params (Key :type "Key Structure"))
  (:`Pressed`
    (`/Game/Blueprints/SideScrollerCharacter.StartMovement` (`self.PCharacter`))))

(event `InputAction|Jump`
  (params (Key :type "Key Structure"))
  (bind _pcharacter (`self.PCharacter`))
  (:`Pressed`
    (if (`self.canJump?`)
      (`Character.Jump` _pcharacter)))
  (:`Released`
    (`Character.StopJumping` _pcharacter)))

(event `Key|Q`
  (params (Key :type "Key Structure"))
  (bind _pcharacter (`self.PCharacter`))
  (:`Pressed`
    (if (`self.canTurn?`)
      (`/Engine/EditorBlueprintResources/StandardMacros.FlipFlop`
        (:`A`
          (set `/Game/Blueprints/SideScrollerCharacter.moveRight?` true _pcharacter))
        (:`B`
          (set `/Game/Blueprints/SideScrollerCharacter.moveRight?` false _pcharacter))))))

(fn `UserConstructionScript`)